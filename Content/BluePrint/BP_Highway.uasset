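; BP_Highway is a world segment for a chicken lane-crossing game that requests the next segment and removes itself.
; When BP_Chiken overlaps TriggerPoint, it calls SpawnWorldAtSpawnPoint on SpawnWorld, then destroys itself.
; RandomizeLoadorTrainorRiver gives ChildActor1 a random road, rail, river or grass lane class, though nothing here calls it.
; Tick applies a zero offset to SpawnWorld, and older LaneState setup logic is left disconnected.
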(event `self.ReceiveTick`
  (params (DeltaSeconds :type "Float (single-precision)"))
  (`self.K2_AddActorLocalOffset` (`self.SpawnWorld`) (0.0 0.0 0.0) true false))

(event `self.TriggerPoint.OnComponentBeginOverlap`
  (params (OverlappedComponent :type "PrimitiveComponent Object Reference") (OtherActor :type "Actor Object Reference") (OtherComp :type "PrimitiveComponent Object Reference") (OtherBodyIndex :type Integer) (bFromSweep :type Boolean) (SweepResult :type "HitResult Structure (by ref)"))
  (cast `/Game/BluePrint/BP_Chiken` OtherActor)
  (`/Game/BluePrint/BP_WorldSpawner.SpawnWorldAtSpawnPoint` (`self.SpawnWorld`))
  (`self.K2_DestroyActor`))

(fn `RandomizeLoadorTrainorRiver`
  (params (Index :type Integer))
  (`ChildActorComponent.SetChildActorClass` (`self.ChildActor1`) (select `int` (`KismetMathLibrary.RandomIntegerInRange` 0 3) :`0` "/Game/BluePrint/BP_Load_right.BP_Load_right_C" :`1` "/Game/BluePrint/BP_rail_train.BP_rail_train_C" :`2` "/Game/BluePrint/BP_River.BP_River_C" :`3` "/Game/BluePrint/BP_Grass_Road.BP_Grass_Road_C" :!type "Actor Class Reference")))

(fn `UserConstructionScript`)