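; BP_rail_train is a rail spawner that sends out BP_Train2 actors and removes them when they reach its trigger box.
; A looping timer, with its interval randomized once at BeginPlay, spawns a train at the Start component on a coin flip.
; A random flag set at BeginPlay gates all spawning, so some instances never spawn; the stored End location is unused.
; The Box overlap destroys any BP_Train2 that enters it.
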(event `self.ReceiveBeginPlay`
  (set `self.Startlocation` (`SceneComponent.K2_GetComponentLocation` (`self.start`)))
  (set `self.Endlocation` (`SceneComponent.K2_GetComponentLocation` (`self.end`)))
  (set `self.startingTrainlocation` (`KismetMathLibrary.RandomBool`))
  (`KismetSystemLibrary.K2_SetTimerDelegate` (delegate `Spawn Train2`) (`KismetMathLibrary.RandomFloatInRange` 2.0 3.0) true))

(event `Spawn Train2`
  (if (`KismetMathLibrary.RandomBool`)
    (if (`self.startingTrainlocation`)
      (`|SpawnActorFromClass` "/Game/BluePrint/BP_Train2.BP_Train2_C" (`KismetMathLibrary.MakeTransform` (`self.Startlocation`) (struct :`Yaw` 180.0)) "Undefined" "OverrideRootScale" null null))))

(event `self.Box.OnComponentBeginOverlap`
  (params (OverlappedComponent :type "PrimitiveComponent Object Reference") (OtherActor :type "Actor Object Reference") (OtherComp :type "PrimitiveComponent Object Reference") (OtherBodyIndex :type Integer) (bFromSweep :type Boolean) (SweepResult :type "HitResult Structure (by ref)"))
  (bind _asbp_train_2 (cast `/Game/BluePrint/BP_Train2` OtherActor))
  (`self.K2_DestroyActor` _asbp_train_2))

(fn `UserConstructionScript`)