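; BP_WorldSpawner builds the level from chained BP_Highway segments at runtime.
; On BeginPlay it spawns a segment at a fixed start, then appends a short initial run, each at the previous segment's SpawnPoint, falling back to the player's location if none is valid.
; Each segment receives a reference back to the spawner and runs its road, train or river randomizer.
; NewestWorld tracks the chain's end for SpawnWorldAtSpawnPoint to extend.
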(event `self.ReceiveBeginPlay`
  (`self.WorldSpawner` (-200.0 0.0 0.0))
  (`self.Spawn Initial World`))

(event `self.ReceiveTick`
  (params (DeltaSeconds :type "Float (single-precision)")))

(fn `Spawn Initial World`
  (for _ (range 3)
    (`/Engine/EditorBlueprintResources/StandardMacros.IsValid` (`self.NewestWorld`)
      (:`Is Valid`
        (`self.SpawnWorldAtSpawnPoint`))
      (:`Is Not Valid`
        (`self.WorldSpawner` (`self.K2_GetActorLocation` (`GameplayStatics.GetPlayerPawn` 0)))))))

(fn `SpawnWorldAtSpawnPoint`
  (`self.WorldSpawner` (`SceneComponent.K2_GetComponentLocation` (`/Game/BluePrint/BP_Highway.SpawnPoint` (`self.NewestWorld`)))))

(fn `UserConstructionScript`)

(fn `WorldSpawner`
  (params (SpawnLocation :type "Vector Structure"))
  (bind _returnvalue (`|SpawnActorFromClass` "/Game/BluePrint/BP_Highway.BP_Highway_C" (`KismetMathLibrary.MakeTransform` SpawnLocation) "Undefined" "OverrideRootScale" null null))
  (bind _output_get (set `self.NewestWorld` _returnvalue))
  (set `/Game/BluePrint/BP_Highway.SpawnWorld` self _output_get)
  (`/Game/BluePrint/BP_Highway.RandomizeLoadorTrainorRiver` _output_get 0))