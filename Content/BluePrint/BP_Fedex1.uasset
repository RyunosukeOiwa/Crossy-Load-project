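; BP_Fedex1 is a moving Fedex obstacle that kills the chicken character when hit.
; It uses a ProjectileMovement component and clears its homing target on BeginPlay.
; A hit on its Box component casts the other actor to BP_Chiken and sets IsDead.
; Unconnected leftover nodes include a player pawn cast and a random choice that would set speed and a truck mesh.
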(event `self.ReceiveBeginPlay`
  (set `ProjectileMovementComponent.HomingTargetComponent` null (`self.ProjectileMovement`)))

(event `self.Box.OnComponentHit`
  (params (HitComponent :type "PrimitiveComponent Object Reference") (OtherActor :type "Actor Object Reference") (OtherComp :type "PrimitiveComponent Object Reference") (NormalImpulse :type "Vector Structure") (Hit :type "HitResult Structure (by ref)"))
  (bind _asbp_chiken (cast `/Game/BluePrint/BP_Chiken` OtherActor))
  (set `/Game/BluePrint/BP_Chiken.IsDead` true _asbp_chiken))

(fn `UserConstructionScript`)