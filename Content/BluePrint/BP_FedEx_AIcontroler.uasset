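; AI controller that sets up the BB_Attack blackboard and reacts to sensing BP_Fedex1 actors.
; BeginPlay initializes the blackboard and calls RunBehaviorTree, with no tree asset specified.
; Perception updates are scanned for a successfully sensed BP_Fedex1, then the loop breaks after a blackboard object write.
; That write looks unfinished: its key name is "None" and no object value is supplied.
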(event `self.ReceiveBeginPlay`
  (bind _blackboardcomponent (`self.UseBlackboard` "/Game/BlackBoard/BB_Attack.BB_Attack"))
  (set `self.Blackboard Component` _blackboardcomponent)
  (`self.RunBehaviorTree` null))

(event `self.AIPerception.OnPerceptionUpdated`
  (params (UpdatedActors :type "Array of Actor Object Reference (by ref)"))
  ;[1 1 1] Comment
  (for _array_element UpdatedActors
    (bind _info (`AIPerceptionComponent.GetActorsPerception` (`self.AIPerception`) _array_element))
    (if (`.bSuccessfullySensed` (break `AIStimulus` (struct)))
      (cast `/Game/BluePrint/BP_Fedex1` _array_element)
      (`BlackboardComponent.SetValueAsObject` (`self.Blackboard Component`) "None" null)
      (break))))

(fn `UserConstructionScript`)