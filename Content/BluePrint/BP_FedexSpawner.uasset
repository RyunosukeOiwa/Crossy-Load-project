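; Spawner Blueprint that creates BP_FedEx_test actors when play begins, starting at the world origin.
; An initial two-pass loop then spawns from NewestFedex's SpawnPoint if valid, otherwise at the player pawn's location.
; The SpawnPoint path passes world scale as the location.
; The spawn function sets NewestFedex to None rather than the new actor, so the following spawner back-reference has no valid target.
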(event `self.ReceiveBeginPlay`
  (`self.FedexSpawner` (0.0 0.0 0.0))
  (`self.SpawnInitialFedex`))

(fn `FedexSpawner`
  (params (`Spawn Location` :type "Vector Structure"))
  (`|SpawnActorFromClass` "/Game/BluePrint/BP_FedEx_test.BP_FedEx_test_C" (`KismetMathLibrary.MakeTransform` `Spawn Location`) "Undefined" "OverrideRootScale" null null)
  (bind _output_get (set `self.NewestFedex` null))
  (set `/Game/BluePrint/BP_FedexRoad.FedexSpawner` self _output_get))

(fn `SpawnFedexAtSpawnPoint`
  (`self.FedexSpawner` (`SceneComponent.K2_GetComponentScale` (`/Game/BluePrint/BP_FedexRoad.SpawnPoint` (`self.NewestFedex`)))))

(fn `SpawnInitialFedex`
  (for _ (range 2)
    (`/Engine/EditorBlueprintResources/StandardMacros.IsValid` (`self.NewestFedex`)
      (:`Is Valid`
        (`self.SpawnFedexAtSpawnPoint`))
      (:`Is Not Valid`
        (`self.FedexSpawner` (`self.K2_GetActorLocation` (`GameplayStatics.GetPlayerPawn` 0)))))))

(fn `UserConstructionScript`)