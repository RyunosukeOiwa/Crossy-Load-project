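; BP_FedexRoad is a road actor that spawns BP_FedEx_test actors and hands them off at a trigger zone.
; A random flag set at BeginPlay decides whether it is a start point, and a looping timer then randomly spawns at SpawnPoint.
; When a BP_FedEx_test enters TriggerZone, the road tells FedexSpawner to spawn one and destroys the arriving actor.
; SpawnRoad is an empty stub.
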(event `self.ReceiveBeginPlay`
  (set `self.SpawnLocation` (`SceneComponent.K2_GetComponentLocation` (`self.SpawnPoint`)))
  (set `self.StartPoint` (`KismetMathLibrary.RandomBool`))
  (`KismetSystemLibrary.K2_SetTimerDelegate` (delegate `SpawnFedex test`) 2.0 true))

(event `SpawnFedex test`
  (if (`KismetMathLibrary.RandomBool`)
    (if (`self.StartPoint`)
      (`|SpawnActorFromClass` "/Game/BluePrint/BP_FedEx_test.BP_FedEx_test_C" (`KismetMathLibrary.MakeTransform` (`self.SpawnLocation`)) "Undefined" "OverrideRootScale" null null))))

(event `self.ReceiveTick`
  (params (DeltaSeconds :type "Float (single-precision)")))

(event `self.trigger zone.OnComponentBeginOverlap`
  (params (OverlappedComponent :type "PrimitiveComponent Object Reference") (OtherActor :type "Actor Object Reference") (OtherComp :type "PrimitiveComponent Object Reference") (OtherBodyIndex :type Integer) (bFromSweep :type Boolean) (SweepResult :type "HitResult Structure (by ref)"))
  (bind _asbp_fed_ex_test (cast `/Game/BluePrint/BP_FedEx_test` OtherActor))
  (`/Game/BluePrint/BP_FedexSpawner.SpawnFedexAtSpawnPoint` (`self.FedexSpawner`))
  (`self.K2_DestroyActor` _asbp_fed_ex_test))

(fn `spawnRoad`)

(fn `UserConstructionScript`)