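; BP_Chiken is a player-controlled chicken whose controller movement stops once when it is hit by BP_Fedex.
; MoveForward and MoveRight feed movement input along swapped right and forward vectors, which Tick consumes as an unswept local offset.
; A half-second cooldown only ever sets Canmove false and does not gate movement.
; RotateToFaceCursor yaws the controller toward the cursor but is not called here, and the WASD rotation logic is disconnected.
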(event `self.ReceiveHit`
  (params (MyComp :type "PrimitiveComponent Object Reference") (Other :type "Actor Object Reference") (OtherComp :type "PrimitiveComponent Object Reference") (bSelfMoved :type Boolean) (HitLocation :type "Vector Structure") (HitNormal :type "Vector Structure") (NormalImpulse :type "Vector Structure") (Hit :type "HitResult Structure (by ref)"))
  (cast `/Game/BluePrint/BP_Fedex` Other)
  (`/Engine/EditorBlueprintResources/StandardMacros.DoOnce` false
    (:`Completed`
      (`Controller.StopMovement` (`self.GetController`)))))

(event `InputAxis|MoveForward`
  (params (AxisValue :type "Float (single-precision)"))
  (`self.Movementcooldown`)
  (`self.AddMovementInput` (`self.GetActorRightVector`) (* AxisValue (`self.MaxSpeed`))))

(event `self.ReceiveBeginPlay`)

(event `InputAxis|MoveRight`
  (params (AxisValue :type "Float (single-precision)"))
  (`self.Movementcooldown`)
  (`self.AddMovementInput` (`self.GetActorForwardVector`) (* AxisValue (`self.MaxSpeed`))))

(event `self.ReceiveTick`
  (params (DeltaSeconds :type "Float (single-precision)"))
  (bind _returnvalue (`self.ConsumeMovementInputVector`))
  (`self.K2_AddActorLocalOffset` (* _returnvalue DeltaSeconds)))

(event `Movementcooldown`
  (`/Engine/EditorBlueprintResources/StandardMacros.DoOnce` false :!label _label
    (:`Completed`
      (set `self.Canmove` false)
      (`KismetSystemLibrary.Delay` 0.5)
      (set `self.Canmove` false)
      (goto _label :!via `Reset`))))

(fn `RotateToFaceCursor`
  (bind _returnvalue (`GameplayStatics.GetPlayerController` 0))
  (bind (_returnvalue_roll _returnvalue_pitch _returnvalue_yaw) (`KismetMathLibrary.BreakRotator` (`KismetMathLibrary.FindLookAtRotation` (`self.K2_GetActorLocation` self) (`.Location` (`GameplayStatics.BreakHitResult` (`PlayerController.GetHitResultUnderCursorByChannel` _returnvalue "TraceTypeQuery1" true))))))
  (`Controller.SetControlRotation` _returnvalue (`KismetMathLibrary.MakeRotator` 0.0 0.0 _returnvalue_yaw)))

(fn `UserConstructionScript`)