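; BP_River is a river lane hazard that spawns BP_Rog actors and marks BP_Chiken dead when it hits HitOutBox.
; BeginPlay rolls a one-time spawn flag and starts a looping timer with an interval randomized once.
; Each tick of that timer has a random chance to spawn at Start, only if the flag is true.
; The Box overlap destroys arriving BP_Rog actors; the cached End location is unused.
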(event `self.ReceiveBeginPlay`
  (set `self.Startlocation` (`SceneComponent.K2_GetComponentLocation` (`self.start`)))
  (set `self.Endlocation` (`SceneComponent.K2_GetComponentLocation` (`self.end`)))
  (set `self.startingcarlocation` (`KismetMathLibrary.RandomBool`))
  (`KismetSystemLibrary.K2_SetTimerDelegate` (delegate `Spawn FedEx`) (`KismetMathLibrary.RandomFloatInRange` 2.0 3.0) true))

(event `Spawn FedEx`
  (if (`KismetMathLibrary.RandomBool`)
    (if (`self.startingcarlocation`)
      (`|SpawnActorFromClass` "/Game/BluePrint/BP_Rog.BP_Rog_C" (`KismetMathLibrary.MakeTransform` (`self.Startlocation`) (struct :`Yaw` 180.0)) "Undefined" "OverrideRootScale" null null))))

(event `self.box.OnComponentBeginOverlap`
  (params (OverlappedComponent :type "PrimitiveComponent Object Reference") (OtherActor :type "Actor Object Reference") (OtherComp :type "PrimitiveComponent Object Reference") (OtherBodyIndex :type Integer) (bFromSweep :type Boolean) (SweepResult :type "HitResult Structure (by ref)"))
  (bind _asbp_rog (cast `/Game/BluePrint/BP_Rog` OtherActor))
  (`self.K2_DestroyActor` _asbp_rog))

(event `self.HitOutBox.OnComponentHit`
  (params (HitComponent :type "PrimitiveComponent Object Reference") (OtherActor :type "Actor Object Reference") (OtherComp :type "PrimitiveComponent Object Reference") (NormalImpulse :type "Vector Structure") (Hit :type "HitResult Structure (by ref)"))
  (bind _asbp_chiken (cast `/Game/BluePrint/BP_Chiken` OtherActor))
  (set `/Game/BluePrint/BP_Chiken.IsDead` true _asbp_chiken))

(fn `UserConstructionScript`)